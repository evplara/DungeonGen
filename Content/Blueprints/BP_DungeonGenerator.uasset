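; Seeded procedural dungeon generator that assembles room modules door to door, with debug keys to generate, reseed or clear.
; From a start room, it randomly picks an open door and a room, then yaws and offsets the candidate to align door sockets.
; A bounds box-overlap test rejects colliding rooms, while placed rooms add their other doors to the open list.
; After reaching the room count or attempt limit, remaining doors get caps.
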(event `self.ReceiveBeginPlay`
  (`InputDeviceLibrary.GetPlayerControllerFromInputDevice` (struct))
  (`self.EnableInput` null))

(event `Key|G`
  (params (Key :type "Key Structure"))
  (:`Pressed`
    (`self.GenerateDungeonMain`)))

(event `Key|C`
  (params (Key :type "Key Structure"))
  (:`Pressed`
    (`self.ClearDungeon`)))

(event `Key|P`
  (params (Key :type "Key Structure"))
  (:`Pressed`
    (set `self.Seed` (`KismetMathLibrary.RandomInteger` 1000))
    (`self.GenerateDungeonMain`)))

(fn `ClearDungeon`
  (for _array_element (`self.SpawnedRooms`)
    (`/Engine/EditorBlueprintResources/StandardMacros.IsValid` _array_element
      (:`Is Valid`
        (`self.K2_DestroyActor` _array_element))))
  (`KismetArrayLibrary.Array_Clear` (`self.SpawnedRooms`))
  (`KismetArrayLibrary.Array_Clear` (`self.OpenDoors`))
  (for _array_element_2 (`self.SpawnedCps`)
    (`/Engine/EditorBlueprintResources/StandardMacros.IsValid` _array_element_2
      (:`Is Valid`
        (`self.K2_DestroyActor` _array_element_2))))
  (`KismetArrayLibrary.Array_Clear` (`self.SpawnedCps`))
  (return))

(fn `CollectOpenDoorsFromRoom`
  (params (Room :type "/Game/Blueprints/BP_RoomModule Object Reference") (ExcludeDoor :type "SceneComponent Object Reference"))
  (`KismetSystemLibrary.PrintString` (`KismetStringLibrary.Concat_StrStr` "OPENED DOORS" (`KismetStringLibrary.Conv_IntToString` (`KismetArrayLibrary.Array_Length` (`self.OpenDoors`)))))
  (`/Engine/EditorBlueprintResources/StandardMacros.IsValid` Room
    (:`Is Valid`
      (for _array_element (`/Game/Blueprints/BP_RoomModule.Door Sockets` Room)
        (if (not (== _array_element ExcludeDoor))
          (`KismetArrayLibrary.Array_Add` (`self.OpenDoors`) (make `/Game/Blueprints/S_OpenDoor` Room _array_element))))
      (return))
    (:`Is Not Valid`
      (return))))

(fn `GenerateDungeonMain`
  (locals (ChosenOpenDoorIndex :type Integer :default 0) (FailCount :type Integer))
  (bind _returnvalue (`KismetArrayLibrary.Array_Length` (`self.OpenDoors`)))
  (`self.ClearDungeon`)
  (`KismetMathLibrary.SetRandomStreamSeed` (`self.Rng`) (`self.Seed`))
  (bind _returnvalue_2 (`|SpawnActorFromClass` (`self.StartRoomClass`) (`KismetMathLibrary.MakeTransform` (0.0 0.0 0.0)) "Undefined" "MultiplyWithRoot" null "NewEnumerator1" null)) ; StartRoom
  (`/Engine/EditorBlueprintResources/StandardMacros.IsValid` _returnvalue_2
    (:`Is Valid`
      (`KismetArrayLibrary.Array_Add` (`self.SpawnedRooms`) _returnvalue_2)
      (`self.CollectOpenDoorsFromRoom` _returnvalue_2)
      (for _ (range (`self.MaxPlacementsAttempts`))
        (if (< (`KismetArrayLibrary.Array_Length` (`self.SpawnedRooms`)) (`self.RoomCount`))
          (if (> _returnvalue 0)
            (bind _returnvalue_3 (`KismetMathLibrary.RandomIntegerInRangeFromStream` (`self.Rng`) 0 (- _returnvalue 1))) ; TargetDoorStruct
            (bind (_success _placedroom _usedcanditdatedoor) (`self.TryPlaceRoomOpenDoor` (`|GetArrayItem` (`self.OpenDoors`) _returnvalue_3)))
            (if _success
              (`KismetArrayLibrary.Array_Remove` (`self.OpenDoors`) (`local.ChosenOpenDoorIndex`))
              (`KismetArrayLibrary.Array_Add` (`self.SpawnedRooms`) _placedroom)
              (`self.CollectOpenDoorsFromRoom` _placedroom _usedcanditdatedoor)
              (`KismetSystemLibrary.PrintString` (`KismetStringLibrary.Concat_StrStr` "SEED:  " (`KismetStringLibrary.Conv_IntToString` (`self.Seed`))))
              (else
                (`/Engine/EditorBlueprintResources/StandardMacros.IncrementInt` (`local.FailCount`))))
            (else
              (break)))
          (else
            (break))))
      (`self.SealUnusedDoors`))
    (:`Is Not Valid`
      (return))))

(fn `SealUnusedDoors`
  (for _array_element (`self.OpenDoors`)
    (bind (_room _door) (break `/Game/Blueprints/S_OpenDoor` _array_element))
    (`/Engine/EditorBlueprintResources/StandardMacros.IsValid` _door
      (:`Is Valid`
        (bind _returnvalue (`|SpawnActorFromClass` (`self.DoorCapClass`) (`KismetMathLibrary.MakeTransform` (+ (`KismetMathLibrary.TransformLocation` (`SceneComponent.K2_GetComponentToWorld` _door)) (* (`SceneComponent.GetForwardVector` _door) 10)) (`SceneComponent.K2_GetComponentRotation` _door)) "Undefined" "MultiplyWithRoot" null null))
        (`KismetArrayLibrary.Array_Add` (`self.SpawnedCps`) _returnvalue))))
  (`KismetArrayLibrary.Array_Clear` (`self.OpenDoors`))
  (return))

(fn `TryPlaceRoomOpenDoor`
  (params (Target :type "/Game/Blueprints/S_OpenDoor Structure"))
  (returns (Success :type Boolean) (PlacedRoom :type "/Game/Blueprints/BP_RoomModule Object Reference") (UsedCanditdateDoor :type "SceneComponent Object Reference"))
  (locals (CandidateDoor :type "SceneComponent Object Reference") (OverlapArray :type "Array of Actor Object Reference"))
  (bind (_room _door) (break `/Game/Blueprints/S_OpenDoor` Target))
  (bind _roomclasses (`self.RoomClasses`))
  (bind _candidateroom (`self.CandidateRoom`))
  (bind _returnvalue (`KismetArrayLibrary.Array_Length` _roomclasses))
  (bind _door_sockets (`/Game/Blueprints/BP_RoomModule.Door Sockets` (`self.CandidateRoom`)))
  (bind _returnvalue_2 (`KismetArrayLibrary.Array_Length` _door_sockets))
  (bind (_origin _boxextent) (`KismetSystemLibrary.GetComponentBounds` (`/Game/Blueprints/BP_RoomModule.BoundsBox` _candidateroom)))
  (`/Engine/EditorBlueprintResources/StandardMacros.IsValid` _door
    (:`Is Valid`
      (if (> _returnvalue 0)
        (bind _returnvalue_3 (`KismetMathLibrary.RandomIntegerInRangeFromStream` (`self.Rng`) 0 (- _returnvalue 1)))
        (bind _returnvalue_4 (`|SpawnActorFromClass` (`|GetArrayItem` _roomclasses _returnvalue_3) (`KismetMathLibrary.MakeTransform` (0.0 0.0 0.0)) "Undefined" "MultiplyWithRoot" null "NewEnumerator1" null))
        (bind _output_get (set `self.CandidateRoom` _returnvalue_4))
        (`/Engine/EditorBlueprintResources/StandardMacros.IsValid` _output_get
          (:`Is Valid`
            (if (> _returnvalue_2 0)
              (bind _returnvalue_5 (`KismetMathLibrary.RandomIntegerInRangeFromStream` (`self.Rng`) 0 (- _returnvalue_2 1)))
              (bind _output_get_2 (set `local.CandidateDoor` (`|GetArrayItem` _door_sockets _returnvalue_5)))
              (`self.K2_AddActorWorldRotation` (`self.CandidateRoom`) (`KismetMathLibrary.MakeRotator` 0.0 0.0 (- (.yaw (`KismetMathLibrary.MakeRotFromX` (* (`SceneComponent.GetForwardVector` _door) -1.0))) (.yaw (`KismetMathLibrary.MakeRotFromX` (`SceneComponent.GetForwardVector` _output_get_2))))) false false)
              (`self.K2_AddActorWorldOffset` _candidateroom (- (`SceneComponent.K2_GetComponentLocation` _door) (`SceneComponent.K2_GetComponentLocation` _output_get_2)) false false)
              (bind _outactors (`KismetSystemLibrary.BoxOverlapActors` _origin _boxextent (`|MakeArray` "ObjectTypeQuery2" "ObjectTypeQuery1" :!type "EObjectTypeQuery Enum") "/Game/Blueprints/BP_RoomModule.BP_RoomModule_C" (`|MakeArray` _room _candidateroom :!type "Actor Object Reference")))
              (set `local.OverlapArray` _outactors)
              (if (> (`KismetArrayLibrary.Array_Length` (`local.OverlapArray`)) 0)
                (`self.K2_DestroyActor` (`self.CandidateRoom`))
                (return false null null)
                (else
                  (return true (`self.CandidateRoom`) (`local.CandidateDoor`))))
              (else
                (`self.K2_DestroyActor` (`self.CandidateRoom`))
                (return false null null))))
          (:`Is Not Valid`
            (return false null null)))
        (else
          (return false null null))))
    (:`Is Not Valid`
      (return false null null))))

(fn `UserConstructionScript`)